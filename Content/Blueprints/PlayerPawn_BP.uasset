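; Player pawn that moves on a spherical planet with its own gravity, using the first Planet_BP found at BeginPlay.
; Each tick it aligns its up axis away from the planet's center and adds velocity toward that center.
; Movement axes add physics velocity along the mesh's forward and right vectors, sharing the gravity's Acceleration value.
; Camera axes yaw the whole actor and pitch the spring arm.
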(event `self.ReceiveBeginPlay`
  (bind _outactors (`GameplayStatics.GetAllActorsOfClass` "/Game/Blueprints/Planet_BP.Planet_BP_C"))
  (set `self.Planet` (`|GetArrayItem` _outactors)))

(event `self.ReceiveTick`
  (params (DeltaSeconds :type "Float (single-precision)"))
  (bind _returnvalue (`KismetMathLibrary.GetForwardVector` (`KismetMathLibrary.FindLookAtRotation` (`self.K2_GetActorLocation` (`self.Planet`)) (`self.K2_GetActorLocation`))))
  (`self.K2_SetActorRotation` (`KismetMathLibrary.MakeRotFromZX` _returnvalue (`SceneComponent.GetForwardVector` (`self.Mesh`))))
  (`PrimitiveComponent.SetPhysicsLinearVelocity` (`self.Mesh`) (* (* _returnvalue -1) (`self.Acceleration`)) true "None"))

(event `InputAxis|Right`
  (params (AxisValue :type "Float (single-precision)"))
  ;[1 1 1] Inputs
  (`PrimitiveComponent.SetPhysicsLinearVelocity` (`self.Mesh`) (* (* (`SceneComponent.GetRightVector` (`self.Mesh`)) AxisValue) (`self.Acceleration`)) true "None"))

(event `InputAxis|Forward`
  (params (AxisValue :type "Float (single-precision)"))
  ;[1 1 1] Inputs
  (`PrimitiveComponent.SetPhysicsLinearVelocity` (`self.Mesh`) (* (* (`SceneComponent.GetForwardVector` (`self.Mesh`)) AxisValue) (`self.Acceleration`)) true "None"))

(event `InputAxis|CameraRight`
  (params (AxisValue :type "Float (single-precision)"))
  ;[1 1 1] Inputs
  (`self.K2_AddActorLocalRotation` (`KismetMathLibrary.MakeRotator` 0.0 0.0 AxisValue)))

(event `InputAxis|CameraUp`
  (params (AxisValue :type "Float (single-precision)"))
  ;[1 1 1] Inputs
  (`SceneComponent.K2_AddLocalRotation` (`self.SpringArm1`) (`KismetMathLibrary.MakeRotator` 0.0 AxisValue) false false))

(fn `UserConstructionScript`)