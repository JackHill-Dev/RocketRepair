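; Actor that orbits a target actor, such as a planet, in a horizontal circle at a set radius.
; Tick accumulates an angle from rotation speed, signed by the Clockwise flag.
; RotateActorAroundPoint adds the starting angle, rotates a radius vector around Z and places the actor relative to the target's current location, only while that target is valid.
; Unconnected nodes for finding other orbiters and lerping speed and radius never run.
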(event `self.ReceiveBeginPlay`
  (set `self.InitialLocation` (`self.K2_GetActorLocation`)))

(event `self.ReceiveTick`
  (params (DeltaSeconds :type "Float (single-precision)"))
  ;[1 1 1] Orbit around planet
  (set `self.CurrentRotation` (+ (`self.CurrentRotation`) (* (* (`self.RotationSpeed`) DeltaSeconds) (`KismetMathLibrary.SelectFloat` 1.0 -1.0 (`self.Clockwise`)))))
  (`self.RotateActorAroundPoint` self (`self.TargetActor`) (`self.InitialLocation`) (`self.Radius`) (`self.StartingAngle`) (`self.CurrentRotation`)))

(fn `RotateActorAroundPoint`
  (params (ActorToRotate :type "Actor Object Reference") (TargetActor :type "Actor Object Reference") (TargetLocation :type "Vector Structure") (Radius :type "Float (double-precision)") (Angle :type "Float (double-precision)") (Rotation :type "Float (double-precision)"))
  (returns (NewParam :type "Vector Structure"))
  (locals (LActorToRotate :type "Actor Object Reference") (LTargetActor :type "Actor Object Reference") (LLocation :type "Vector Structure") (LocalRadius :type "Float (double-precision)") (LAngle :type "Float (double-precision)") (LRate :type "Float (double-precision)"))
  (set `local.LActorToRotate` ActorToRotate)
  (set `local.LTargetActor` TargetActor)
  (set `local.LLocation` TargetLocation)
  (set `local.LocalRadius` Radius)
  (set `local.LAngle` Angle)
  (set `local.LRate` Rotation)
  (`/Engine/EditorBlueprintResources/StandardMacros.IsValid` (`local.LTargetActor`)
    (:`Is Valid`
      (set `local.LLocation` (`self.K2_GetActorLocation` (`local.LTargetActor`)))
      (`self.K2_SetActorLocation` (`local.LActorToRotate`) (+ (`local.LLocation`) (`KismetMathLibrary.RotateAngleAxis` (`KismetMathLibrary.MakeVector` (`local.LocalRadius`)) (+ (`local.LAngle`) (`local.LRate`)) (0.0 0.0 1.0))) false false)
      (return (`local.LLocation`)))))

(fn `UserConstructionScript`)