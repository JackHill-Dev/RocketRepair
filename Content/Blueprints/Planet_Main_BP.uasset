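; Planet actor Blueprint that sizes its Planet component to a radius specified in meters.
; The construction script converts the radius to Unreal units and divides it by the component's bounds X extent to set a uniform world scale.
; GetSurfaceLocationAndNormalAt is an unimplemented stub that takes a location, and the event graph holds only disabled default events.
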(fn `GetSurfaceLocationAndNormalAt`
  (params (Location :type "Array of Vector Structure"))
  (returns (SurfaceLocation :type "Array of Vector Structure") (SurfaceNormal :type "Array of Vector Structure"))
  (return))

(fn `UserConstructionScript`
  (bind _output_get (set `self.RadiusInUnits` (* (`self.RadiusInMeters`) 100.0)))
  (`SceneComponent.SetWorldScale3D` (`self.Planet`) (`KismetMathLibrary.Conv_DoubleToVector` (/ _output_get (.x (`.BoxExtent` (`KismetSystemLibrary.GetComponentBounds` (`self.Planet`))))))))